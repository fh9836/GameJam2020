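; Camera Blueprint that positions and aims its camera relative to a LocationTarget.
; E_Init starts follow, where a looping 0.005-second timer drives the camera update instead of Tick.
; Each update places the camera between the spring arm and target by FollowSpeed, and blends spring arm rotation toward a look-at rotation by LookSpeed.
; Both speeds act as fixed lerp alphas from the spring arm transform, without delta-time scaling.
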(event `E_Init`
  (`self.E_StartFollow`))

(event `E_StartFollow`
  (bind _returnvalue (`KismetSystemLibrary.K2_SetTimerDelegate` (delegate `E_UpdateCameraPosition`) 0.005 true))
  (set `self.Timer` _returnvalue))

(event `E_UpdateCameraPosition`
  (bind _springarm (`self.SpringArm`))
  (bind _returnvalue (`SceneComponent.K2_GetComponentLocation` _springarm))
  (`SceneComponent.K2_SetWorldLocationAndRotation` (`self.Camera`) (`KismetMathLibrary.VLerp` _returnvalue (`SceneComponent.K2_GetComponentLocation` (`Actor.RootComponent` (`self.LocationTarget`))) (`self.FollowSpeed`)) (`KismetMathLibrary.RLerp` (`SceneComponent.K2_GetComponentRotation` _springarm) (`KismetMathLibrary.FindLookAtRotation` _returnvalue (`SceneComponent.K2_GetComponentLocation` (`Actor.RootComponent` (`self.LocationTarget`)))) (`self.LookSpeed`) true) false false))

(fn `UserConstructionScript`)