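; Test object that a player can pick up, carry, detach or consume.
; Interaction attaches the actor to the player, keeping world location and snapping rotation, then registers itself as the player's attached object and stores the holder.
; Detach is delegated to the holder's EDetach event, and Consume destroys the actor.
; GetHeldItem is an empty stub, and an Attached setter in the event graph is unwired.
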(event `/Game/Jammy/Blueprints/I_interactions.DetachAction`
  (`self.F_Detach`))

(event `/Game/Jammy/Blueprints/I_interactions.Interaction`
  (params (`Hit Comp` :type "ActorComponent Object Reference") (Player :type "/Game/Jammy/Blueprints/B_Robit_Player Object Reference"))
  (`self.K2_AttachToActor` self Player "None" "KeepWorld" "SnapToTarget" "KeepRelative" true)
  (set `/Game/Jammy/Blueprints/B_Robit_Player.Attached` true Player)
  (set `/Game/Jammy/Blueprints/B_Robit_Player.attachedObject` self Player)
  (set `self.HeldBy` Player))

(fn `Consume`
  (`self.K2_DestroyActor`))

(fn `F_Detach`
  (`/Game/Jammy/Blueprints/B_Robit_Player.E_Detach` (`self.HeldBy`)))

(fn `GetHeldItem`
  (returns (HeldItem :type "/Game/Jammy/Blueprints/testobject Object Reference"))
  (return null))

(fn `UserConstructionScript`)