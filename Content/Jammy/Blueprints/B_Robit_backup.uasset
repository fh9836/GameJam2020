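; Player-controlled robot pawn (Robit), apparently a backup copy, that moves around and interacts with objects.
; Axis input drives interpolated turning and forward/back movement, both blocked while MovingToRoom is set through the Input event, which also toggles Box activation.
; The A button detaches any held object, otherwise line-traces from the Arrow with debug drawing and sends InteractionMessage to the hit actor.
; Pickup attach logic is disconnected and GetHeldItem is empty.
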(event `self.ReceiveBeginPlay`
  (bind _asrobit_controller (cast `/Game/Jammy/Blueprints/RobitController` (`self.GetController`)))
  (set `self.Robit Controller` _asrobit_controller))

(event `InputAxisKey|Gamepad_LeftX`
  (params (AxisValue :type "Float (single-precision)")))

(event `/Game/Jammy/Blueprints/I_Robit.Move Rot`
  (params (Axis :type "Float (single-precision)"))
  (bind _box (`self.Box`))
  ;[1 1 1] Movement
  (if (not (`self.MovingToRoom`))
    (`self.K2_SetActorRelativeRotation` (`KismetMathLibrary.RInterpTo` (`SceneComponent.RelativeRotation` _box) (`KismetMathLibrary.ComposeRotators` (`SceneComponent.RelativeRotation` _box) (`KismetMathLibrary.MakeRotator` 0.0 0.0 (* Axis (`self.Rot Rate`)))) (`GameplayStatics.GetWorldDeltaSeconds`) 20.0))))

(event `InputAxisKey|Gamepad_LeftY`
  (params (AxisValue :type "Float (single-precision)")))

(event `/Game/Jammy/Blueprints/I_Robit.Move Forward/Back`
  (params (Axis :type "Float (single-precision)"))
  ;[1 1 1] Movement
  (if (not (`self.MovingToRoom`))
    (`self.AddMovementInput` (`KismetMathLibrary.GetForwardVector` (`self.K2_GetActorRotation`)) Axis)))

(event `InputAction|A Button`
  (params (Key :type "Key Structure"))
  (bind _arrow (`self.Arrow`))
  (bind _location (.location (`SceneComponent.K2_GetComponentToWorld` _arrow)))
  (:`Pressed`
    (if (`self.Attached`)
      (if true
        (`self.K2_DetachFromActor` (`self.attachedObject`) "KeepWorld" "KeepWorld" "KeepWorld")
        (set `self.attachedObject` null)
        (set `self.Attached` false))
      (else
        (bind (_outhit _returnvalue) (`KismetSystemLibrary.LineTraceSingleForObjects` :`Start` _location :`End` (+ _location (* (`SceneComponent.GetForwardVector` _arrow) 100)) :`ObjectTypes` (`self.Objects`) :`DrawDebugType` "Persistent"))
        (if _returnvalue
          (bind (_bblockinghit _binitialoverlap _time _distance _location_2 _impactpoint _normal _impactnormal _physmat _hitactor _hitcomponent) (`GameplayStatics.BreakHitResult` _outhit))
          (message `/Game/Jammy/Blueprints/I_interactions.Interaction` _hitactor _hitcomponent null))))))

(event `/Game/Jammy/Blueprints/I_Robit.Input`
  (params (Input :type Boolean))
  (if Input
    (set `self.MovingToRoom` true)
    (`/Engine/EditorBlueprintResources/StandardMacros.DoOnce` false
      (:`Completed`
        (`ActorComponent.ToggleActive` (`self.Box`))))
    (else
      (set `self.MovingToRoom` false)
      (`/Engine/EditorBlueprintResources/StandardMacros.DoOnce` false
        (:`Completed`
          (`ActorComponent.ToggleActive` (`self.Box`)))))))

(fn `GetHeldItem`
  (returns (HeldItem :type "/Game/Jammy/Blueprints/testobject Object Reference"))
  (return null))

(fn `UserConstructionScript`)