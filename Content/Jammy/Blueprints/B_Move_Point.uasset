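; B_Move_Point is a two-way transit actor that carries the player along a spline between two interaction points.
; The construction script places Point1 and Point2 at the spline's ends.
; Interaction checks for the "Point 1" tag to pick direction, toggles InputMessage around the trip, and uses DoOnce-guarded timelines to set player location and rotation along the spline.
; The return trip adds 180 degrees of yaw to face travel direction.
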(event `self.Point 1.OnComponentHit`
  (params (HitComponent :type "PrimitiveComponent Object Reference") (OtherActor :type "Actor Object Reference") (OtherComp :type "PrimitiveComponent Object Reference") (NormalImpulse :type "Vector Structure") (Hit :type "HitResult Structure (by ref)")))

(event `/Game/Jammy/Blueprints/I_interactions.Interaction`
  (params (`Hit Comp` :type "ActorComponent Object Reference") (Player :type "/Game/Jammy/Blueprints/B_Robit_Player Object Reference"))
  (bind _spline (`self.Spline`))
  (bind _spline_2 (`self.Spline`))
  (if (`self.ActorHasTag` Player "Player")
    (if (`ActorComponent.ComponentHasTag` `Hit Comp` "Point 1")
      (message `/Game/Jammy/Blueprints/I_Robit.Input` Player true)
      (`/Engine/EditorBlueprintResources/StandardMacros.DoOnce` false :!label _label
        (:`Completed`
          (`KismetSystemLibrary.Delay` 0.2)
          (bind (_direction _alpha) (`Timeline|Room Move` :!via `PlayFromStart`)
            (:`Update`
              (bind (_returnvalue_location _returnvalue_rotation) (`KismetMathLibrary.BreakTransform` (`SplineComponent.GetTransformAtDistanceAlongSpline` (`self.Spline`) (`KismetMathLibrary.Lerp` (`SplineComponent.GetDistanceAlongSplineAtSplinePoint` _spline_2 0) (`SplineComponent.GetSplineLength` _spline_2) _alpha) "World" false)))
              (`self.K2_SetActorLocationAndRotation` Player _returnvalue_location _returnvalue_rotation false false))
            (:`Finished`
              (message `/Game/Jammy/Blueprints/I_Robit.Input` Player false)
              (goto _label :!via `Reset`)))))
      (else
        (message `/Game/Jammy/Blueprints/I_Robit.Input` Player true)
        (`/Engine/EditorBlueprintResources/StandardMacros.DoOnce` false :!label _label_2
          (:`Completed`
            (`KismetSystemLibrary.Delay` 0.2)
            (bind (_direction_2 _alpha_2) (`Timeline|Timeline_0` :!via `PlayFromStart`)
              (:`Update`
                (bind (_returnvalue_location_2 _returnvalue_rotation_2) (`KismetMathLibrary.BreakTransform` (`SplineComponent.GetTransformAtDistanceAlongSpline` (`self.Spline`) (`KismetMathLibrary.Lerp` (`SplineComponent.GetSplineLength` _spline) (`SplineComponent.GetDistanceAlongSplineAtSplinePoint` _spline 0) _alpha_2) "World" false)))
                (`self.K2_SetActorLocationAndRotation` Player _returnvalue_location_2 (`KismetMathLibrary.MakeRotator` (.roll _returnvalue_rotation_2) (.pitch _returnvalue_rotation_2) (+ (.yaw _returnvalue_rotation_2) 180.0)) false false))
              (:`Finished`
                (message `/Game/Jammy/Blueprints/I_Robit.Input` Player false)
                (goto _label_2 :!via `Reset`)))))))))

(fn `GetHeldItem`
  (returns (HeldItem :type "/Game/Jammy/Blueprints/testobject Object Reference"))
  (return null))

(fn `UserConstructionScript`
  (bind _spline (`self.Spline`))
  (`SceneComponent.K2_SetWorldLocation` (`self.Point 1`) (`SplineComponent.GetLocationAtSplinePoint` _spline 0 "World") false false)
  (`SceneComponent.K2_SetWorldLocation` (`self.Point 2`) (`SplineComponent.GetLocationAtSplinePoint` _spline (`SplineComponent.GetNumberOfSplinePoints` _spline) "World") false false))