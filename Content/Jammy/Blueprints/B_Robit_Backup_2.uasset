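; Player-controlled robot pawn that moves, interacts with pickups and doors, and can release a carried object, viewed through a CameraSpot camera.
; Axis input drives FloatingPawnMovement, and rotation eases toward the velocity direction.
; The A button traces for pickups when empty-handed, or doors when carrying, sending InteractionMessage on a hit and detaching if no door is found.
; An Input event sets MovingToRoom and toggles Box; GetHeldItem exposes the carried testobject.
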(event `self.ReceiveBeginPlay`
  (`|ExecutionSequence`
    (:`then_0`
      (bind _asrobit_controller (cast `/Game/Jammy/Blueprints/RobitController` (`self.GetController`)))
      (set `self.Robit Controller` _asrobit_controller))
    (:`then_1`
      (`PlayerController.SetViewTargetWithBlend` (`GameplayStatics.GetPlayerController` 0) (`ChildActorComponent.ChildActor` (`self.Camera Spot`)) 0.0 "VTBlend_Linear" 0.0 false))))

(event `/Game/Jammy/Blueprints/I_Robit.Move Forward/Back`
  (params (Axis :type "Float (single-precision)"))
  (bind _velocity (`MovementComponent.Velocity` (`self.FloatingPawnMovement`)))
  ;[1 1 1] Movement
  (`PawnMovementComponent.AddInputVector` (`self.FloatingPawnMovement`) (`KismetMathLibrary.MakeVector` Axis (stale `/Game/Jammy/Blueprints/I_Robit.Move Rot` Axis)) false :!label _label)
  (if (> (`KismetMathLibrary.VSize` _velocity) 0.0)
    (`self.K2_SetActorRelativeRotation` (`KismetMathLibrary.RInterpTo` (`SceneComponent.RelativeRotation` (`self.Robit`)) (`KismetMathLibrary.Conv_VectorToRotator` (`KismetMathLibrary.Normal` _velocity)) (`GameplayStatics.GetWorldDeltaSeconds`) 2.0))))

(event `/Game/Jammy/Blueprints/I_Robit.Move Rot`
  (params (Axis :type "Float (single-precision)"))
  ;[1 1 1] Movement
  (goto _label))

(event `InputAction|A Button`
  (params (Key :type "Key Structure"))
  (bind _interaction_2 (`self.Interaction 2`))
  (bind _interaction_1 (`self.Interaction 1`))
  (bind _location (.location (`SceneComponent.K2_GetComponentToWorld` _interaction_1)))
  (bind _location_2 (.location (`SceneComponent.K2_GetComponentToWorld` _interaction_2)))
  (:`Pressed`
    (if (`self.Attached`)
      (bind (_outhit _returnvalue) (`KismetSystemLibrary.LineTraceSingleForObjects` :`Start` _location_2 :`End` (+ _location_2 (* (`SceneComponent.GetForwardVector` _interaction_2) 100)) :`ObjectTypes` (`self.Doors`) :`DrawDebugType` "Persistent" :`TraceColor` (struct :`R` 1.0 :`G` 0.940353 :`A` 1.0) :`TraceHitColor` (struct :`R` 0.041467 :`G` 1.0 :`A` 1.0)))
      (if _returnvalue
        (bind (_bblockinghit _binitialoverlap _time _distance _location_3 _impactpoint _normal _impactnormal _physmat _hitactor _hitcomponent) (`GameplayStatics.BreakHitResult` _outhit))
        (message `/Game/Jammy/Blueprints/I_interactions.Interaction` _hitactor _hitcomponent null)
        (else
          (`self.E_Detach`)))
      (else
        (bind (_outhit_2 _returnvalue_2) (`KismetSystemLibrary.LineTraceSingleForObjects` :`Start` _location :`End` (+ _location (* (`SceneComponent.GetForwardVector` _interaction_1) 100)) :`ObjectTypes` (`self.PickupObjects`) :`DrawDebugType` "Persistent"))
        (if _returnvalue_2
          (bind (_bblockinghit_2 _binitialoverlap_2 _time_2 _distance_2 _location_4 _impactpoint_2 _normal_2 _impactnormal_2 _physmat_2 _hitactor_2 _hitcomponent_2) (`GameplayStatics.BreakHitResult` _outhit_2))
          (message `/Game/Jammy/Blueprints/I_interactions.Interaction` _hitactor_2 _hitcomponent_2 null))))))

(event `E_Detach`
  (`self.K2_DetachFromActor` (`self.attachedObject`) "KeepWorld" "KeepWorld" "KeepWorld")
  (set `self.attachedObject` null)
  (set `self.Attached` false))

(event `/Game/Jammy/Blueprints/I_Robit.Input`
  (params (Input :type Boolean))
  (if Input
    (set `self.MovingToRoom` true)
    (`/Engine/EditorBlueprintResources/StandardMacros.DoOnce` false
      (:`Completed`
        (`ActorComponent.ToggleActive` (`self.Box`))))
    (else
      (set `self.MovingToRoom` false)
      (`/Engine/EditorBlueprintResources/StandardMacros.DoOnce` false
        (:`Completed`
          (`ActorComponent.ToggleActive` (`self.Box`)))))))

(fn `GetHeldItem`
  (returns (HeldItem :type "/Game/Jammy/Blueprints/testobject Object Reference"))
  (bind _attachedobject (`self.attachedObject`))
  (`/Engine/EditorBlueprintResources/StandardMacros.IsValid` _attachedobject
    (:`Is Valid`
      (bind _astestobject (cast `/Game/Jammy/Blueprints/testobject` _attachedobject))
      (return _astestobject))
    (:`Is Not Valid`
      (return null))))

(fn `UserConstructionScript`)